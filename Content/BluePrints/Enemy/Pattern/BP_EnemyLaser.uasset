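; Golem boss laser beam attack that constantly aims at the player and grows in length up to a distance cap.
; A per-tick visibility trace, ignoring the boss, places the Niagara or particle beam end and impact effect.
; Continuous contact damages the player at half-second intervals.
; Holding on one rock pillar for two seconds destroys it, tells GolemBossEnemy to end the attack, stops the sound and destroys the laser.
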(event EventBeginPlay
  (Effects|Components|ParticleSystem|SetColorParameter (Variables|Default|GetLaserImpact) "Colour" "(R=0.049932,G=1.000000,B=0.000000,A=1.000000)")
  (bind _returnvalue (Audio|SpawnSound2D "/Game/BluePrints/EnemySFX/Raser.Raser" 1.0 1.0 0.0 0))
  (Variables|Default|SetSound _returnvalue))

(event EventTick
  (params (DeltaSeconds :type Float%20%28single-precision%29))
  (bind _returnvalue (Transformation|GetActorLocation))
  (bind _laserimpact (Variables|Default|GetLaserImpact))
  (Utilities|FlowControl|Sequence
    (:then_0
      (Variables|Default|SetTraceEnd (+ _returnvalue (* (Math|Vector|Normalize (- (Transformation|GetActorLocation (Game|Player|GetPlayerPawn 0)) (Transformation|GetActorLocation))) (Variables|Default|GetDistance))))
      (bind _returnvalue_2 (Actor|GetActorOfClass "/Script/Gunfire.GolemBossEnemy"))
      (bind _outhit (Collision|LineTraceByChannel _returnvalue (+ _returnvalue (* (Math|Vector|Normalize (- (Transformation|GetActorLocation (Game|Player|GetPlayerPawn 0)) (Transformation|GetActorLocation))) (Variables|Default|GetDistance))) "TraceTypeQuery1" false (Utilities|Array|MakeArray _returnvalue_2) "None"))
      (Utilities|FlowControl|Sequence
        (:then_0
          (bind _output_get (Variables|Default|SetHit (.bblockinghit _outhit)))
          (Effects|Components|ParticleSystem|SetVectorParameter (Variables|Default|GetLaser) "BeamEnd" (select _output_get (.location _outhit) (Variables|Default|GetTraceEnd)))
          (Rendering|SetVisibility _laserimpact (Variables|Default|GetHit) false)
          (Transformation|SetWorldLocation _laserimpact (.location _outhit) false false))
        (:then_1
          (bind _astpsplayer (Utilities|Casting|CastToTPSPlayer (.hitactor _outhit))
            (:then
              (bind _output_get_2 (Variables|Default|SetPlayerTargetedTime (+ (Variables|Default|GetPlayerTargetedTime) (Utilities|Time|GetWorldDeltaSeconds))))
              (if (> _output_get_2 0.5)
                (Game|Damage|ApplyDamage _astpsplayer (Variables|Default|GetDamage) 0 0)
                (Variables|Default|SetPlayerTargetedTime 0.0)))
            (:CastFailed
              (Variables|Default|SetPlayerTargetedTime 0.0))))
        (:then_2
          (bind _asbp_enemy_rock_pillar (Utilities|Casting|CastToBP_EnemyRockPillar (.hitactor _outhit))
            (:then
              (if (== _asbp_enemy_rock_pillar (Variables|Default|GetTargetedRock))
                (bind _output_get_3 (Variables|Default|SetRockTargetedTime (+ (Variables|Default|GetRockTargetedTime) (Utilities|Time|GetWorldDeltaSeconds))))
                (if (> _output_get_3 2.0)
                  (Variables|Default|SetRockTargetedTime 0.0)
                  (Default|DestroyRock _asbp_enemy_rock_pillar)
                  (bind _returnvalue_3 (Actor|GetActorOfClass "/Script/Gunfire.GolemBossEnemy"))
                  (Class|GolemBossEnemy|EndLaserAttack _returnvalue_3)
                  (Audio|Components|Audio|Stop (Variables|Default|GetSound))
                  (Actor|DestroyActor))
                (else
                  (Variables|Default|SetTargetedRock _asbp_enemy_rock_pillar)
                  (Variables|Default|SetRockTargetedTime 0.0))))
            (:CastFailed
              (Variables|Default|SetRockTargetedTime 0.0))))))
    (:then_1
      (if (< (Variables|Default|GetDistance) 5e+03)
        (Variables|Default|SetDistance (+ (Variables|Default|GetDistance) (* (Variables|Default|GetSpeed) DeltaSeconds)))))))

(fn ConstructionScript)