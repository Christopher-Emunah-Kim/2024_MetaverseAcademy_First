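; BP_Laser is an enemy pattern actor that renders a Niagara laser beam aimed at the player pawn.
; Each tick it line-traces on Visibility toward the player's current position over a length that grows at Speed up to a fixed cap.
; The beam ends at the blocking hit or trace end, with an impact effect shown only on hits.
; It tints both effects green at BeginPlay and applies no damage itself.
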(event EventBeginPlay
  (Effects|Components|ParticleSystem|SetColorParameter (Variables|Default|GetNiagaraLaser) "Colour" "(R=0.049932,G=1.000000,B=0.000000,A=1.000000)"))

(event Collision|EventActorBeginOverlap
  (params (OtherActor :type Actor%20Object%20Reference)))

(event EventTick
  (params (DeltaSeconds :type Float%20%28single-precision%29))
  (bind _returnvalue (Transformation|GetActorLocation))
  (bind _niagaralaserimpact (Variables|Default|GetNiagaraLaserImpact))
  (Utilities|FlowControl|Sequence
    (:then_0
      (Variables|Default|SetTraceEnd (+ _returnvalue (* (Math|Vector|Normalize (- (Transformation|GetActorLocation (Game|Player|GetPlayerPawn 0)) (Transformation|GetActorLocation))) (Variables|Default|GetDistance))))
      (bind _outhit (Collision|LineTraceByChannel _returnvalue (+ _returnvalue (* (Math|Vector|Normalize (- (Transformation|GetActorLocation (Game|Player|GetPlayerPawn 0)) (Transformation|GetActorLocation))) (Variables|Default|GetDistance))) "TraceTypeQuery1" false 0 "None"))
      (bind _output_get (Variables|Default|SetHit (.bblockinghit _outhit)))
      (Effects|Components|ParticleSystem|SetVectorParameter (Variables|Default|GetNiagaraLaser) "BeamEnd" (select _output_get (.location _outhit) (Variables|Default|GetTraceEnd)))
      (Rendering|SetVisibility _niagaralaserimpact (Variables|Default|GetHit) false)
      (Transformation|SetWorldLocation _niagaralaserimpact (.location _outhit) false false))
    (:then_1
      (if (< (Variables|Default|GetDistance) 5e+03)
        (Variables|Default|SetDistance (+ (Variables|Default|GetDistance) (* (Variables|Default|GetSpeed) DeltaSeconds)))))))

(fn ConstructionScript)