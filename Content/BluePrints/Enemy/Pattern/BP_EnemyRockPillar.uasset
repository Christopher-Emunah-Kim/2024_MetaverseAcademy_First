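; Enemy rock pillar attack that telegraphs with a circle indicator, then rises and can later explode.
; After a delay, the hidden cube becomes visible and collidable, damages the player via sphere trace, and lerps toward Pos on Tick with a rapidly growing alpha.
; DoExplosion triggers a second indicator and red material, then a timer spawns explosions, repeats the area damage and destroys the actor.
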(event Custom|ShowRock
  (bind _returnvalue (Transformation|GetActorLocation))
  (Rendering|SetVisibility (Variables|Default|GetCube) true false)
  (Variables|Default|SetbSummon true)
  (Collision|SetCollisionEnabled (Variables|Default|GetCube) "QueryAndPhysics")
  (CallFunction|SphereDamage _returnvalue _returnvalue))

(event Custom|DestroyMe
  (bind _returnvalue (Game|SpawnActorfromClass "/Game/BluePrints/Enemy/Indicator/BP_CircleIndicator.BP_CircleIndicator_C" (Transformation|GetActorTransform) "Undefined" "MultiplyWithRoot" 0 0))
  (Variables|/Script/Gunfire.SkillIndicator|SetCastingTime _returnvalue 1.0)
  (Variables|/Script/Gunfire.SkillIndicator|SetDestroyTime _returnvalue 1.5)
  (Utilities|Time|SetTimerbyEvent (delegate Custom|CustomEvent) 1.0)
  (Rendering|Material|SetMaterial (Variables|Default|GetCube) 0 "/AnimationSharing/AnimSharingRed.AnimSharingRed"))

(event Custom|CustomEvent
  (bind _returnvalue (Transformation|GetActorTransform))
  (bind _returnvalue_2 (Transformation|GetActorLocation))
  (Game|SpawnActorfromClass "/Game/BluePrints/Enemy/Pattern/BP_Explosion.BP_Explosion_C" _returnvalue "Undefined" "MultiplyWithRoot" 0 0)
  (Game|SpawnActorfromClass "/Game/BluePrints/Enemy/Pattern/BP_EarthExplosion.BP_EarthExplosion_C" _returnvalue "Undefined" "MultiplyWithRoot" 0 0)
  (CallFunction|SphereDamage _returnvalue_2 _returnvalue_2)
  (Audio|PlaySoundatLocation "/Game/BluePrints/EnemySFX/BrokenRock.BrokenRock" _returnvalue_2 "0, 0, 0" 0.4 0.4 0.0 0 0 0 0)
  (Actor|DestroyActor))

(event EventBeginPlay
  (Utilities|FlowControl|Sequence
    (:then_0
      (bind _returnvalue (Game|SpawnActorfromClass "/Game/BluePrints/Enemy/Indicator/BP_CircleIndicator.BP_CircleIndicator_C" (Transformation|GetActorTransform) "Undefined" "MultiplyWithRoot" 0 0))
      (Variables|/Script/Gunfire.SkillIndicator|SetCastingTime _returnvalue 2.0)
      (Audio|PlaySoundatLocation "/Game/BluePrints/EnemySFX/Rock.Rock" (Transformation|GetActorLocation) "0, 0, 0" 0.2 0.2 0.0 0 0 0 0))
    (:then_1
      (Utilities|Time|SetTimerbyEvent (delegate Custom|ShowRock) 2.0))))

(event Collision|EventActorBeginOverlap
  (params (OtherActor :type Actor%20Object%20Reference)))

(event EventDoExplosion
  (CallFunction|DestroyRock))

(event EventTick
  (params (DeltaSeconds :type Float%20%28single-precision%29))
  (bind _cube (Variables|Default|GetCube))
  (bind _returnvalue (Transformation|GetRelativeTransform _cube))
  (Utilities|FlowControl|Sequence
    (:then_0
      (if (Variables|Default|GetbSummon)
        (if (< (Math|Vector|VectorLength (- (.location _returnvalue) (Variables|Default|GetPos))) 0.1)
          (Variables|Default|SetbSummon false)
          (else
            (bind _output_get (Variables|Default|SetCurrentTime (+ (* (Variables|Default|GetCurrentTime) 2.0) DeltaSeconds)))
            (Transformation|SetRelativeTransform (Variables|Default|GetCube) (Math|Transform|MakeTransform (Math|Vector|Lerp(Vector) (.location _returnvalue) (Variables|Default|GetPos) (Math|Float|Clamp(Float) _output_get)) (.rotation _returnvalue) (.scale _returnvalue)) false false)))))))

(fn ConstructionScript)

(fn DestroyRock
  (CallFunction|DestroyMe))

(fn SphereDamage
  (params (End :type Vector) (Start :type Vector))
  (bind _outhits (Collision|MultiSphereTraceByChannel Start End 4e+02 "TraceTypeQuery1" false 0 "None"))
  (bind _array_element (Utilities|Array|ForEachLoopwithBreak _outhits :!label _label)
    (:LoopBody
      (if (.bBlockingHit (Collision|BreakHitResult _array_element))
        (bind _astpsplayer (Utilities|Casting|CastToTPSPlayer (.HitActor (Collision|BreakHitResult _array_element))))
        (Game|Damage|ApplyDamage _astpsplayer 5e+01 0 0)
        (goto _label Break)))))