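; BP_EnemyChasingStone is an enemy stone that tumbles and, after a short delay, homes in on the player.
; BeginPlay picks a random per-axis spin and starts a timer that enables chasing.
; Tick applies the spin every frame and, while chasing, moves the stone straight toward player pawn 0 without sweep.
; Any damage only spawns a BP_DamageAmt actor carrying the amount; no health is tracked here.
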(event Custom|CustomEvent
  (Variables|Default|SetbChase true))

(event EventBeginPlay
  (bind _returnvalue (Math|Random|RandomFloatinRange 0.0 1.0))
  (Utilities|FlowControl|Sequence
    (:then_0
      (Utilities|Time|SetTimerbyEvent (delegate Custom|CustomEvent) 2.0))
    (:then_1
      (Variables|Default|SetRotationSpeed (Math|Rotator|MakeRotator _returnvalue _returnvalue _returnvalue)))))

(event EventTick
  (params (DeltaSeconds :type Float%20%28single-precision%29))
  (Utilities|FlowControl|Sequence
    (:then_0
      (Transformation|AddActorLocalRotation (Variables|Default|GetRotationSpeed) false false))
    (:then_1
      (if (Variables|Default|GetbChase)
        (Transformation|SetActorLocation (+ (Transformation|GetActorLocation) (* (Math|Vector|Normalize (- (Transformation|GetActorLocation (Game|Player|GetPlayerPawn 0)) (Transformation|GetActorLocation))) (Variables|Default|GetSpeed) DeltaSeconds)) false false)))))

(event Game|Damage|EventAnyDamage
  (params (Damage :type Float%20%28single-precision%29) (DamageType :type Damage%20Type%20Object%20Reference) (InstigatedBy :type Controller%20Object%20Reference) (DamageCauser :type Actor%20Object%20Reference))
  (Game|SpawnActorfromClass "/Game/BluePrints/Enemy/BP_DamageAmt.BP_DamageAmt_C" (Math|Transform|MakeTransform (Transformation|GetActorLocation) "0, 0, 0" "1.000000,1.000000,1.000000") "Undefined" "MultiplyWithRoot" 0 Damage 0))

(fn ConstructionScript)