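; Melee sword enemy Blueprint that adds damage feedback and a camera-facing health bar.
; AnyDamage spawns a BP_DamageAmt actor at the enemy's location, passing it the damage amount to represent the hit.
; Tick billboards HPBarWidget by rotating it toward the player camera manager's location every frame.
; No attack, movement or health logic appears in these graphs.
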(event EventBeginPlay)

(event Collision|EventActorBeginOverlap
  (params (OtherActor :type Actor%20Object%20Reference)))

(event EventTick
  (params (DeltaSeconds :type Float%20%28single-precision%29))
  (bind _hpbarwidget (Variables|Default|GetHPBarWidget))
  ;[1 1 1] Target-me로 HP Widget가 돌아가도록 빌보드 처리
  (Transformation|SetWorldRotation _hpbarwidget (Class|KismetMathLibrary|QuatRotator (Math|Conversions|ToQuaternion(Rotator) (- (Transformation|GetActorLocation (Game|GetPlayerCameraManager 0)) (Transformation|GetWorldLocation _hpbarwidget)))) false false))

(event Game|Damage|EventAnyDamage
  (params (Damage :type Float%20%28single-precision%29) (DamageType :type Damage%20Type%20Object%20Reference) (InstigatedBy :type Controller%20Object%20Reference) (DamageCauser :type Actor%20Object%20Reference))
  (Game|SpawnActorfromClass "/Game/BluePrints/Enemy/BP_DamageAmt.BP_DamageAmt_C" (Math|Transform|MakeTransform (Transformation|GetActorLocation) "0, 0, 0" "1.000000,1.000000,1.000000") "Undefined" "MultiplyWithRoot" 0 Damage 0))

(fn ConstructionScript)