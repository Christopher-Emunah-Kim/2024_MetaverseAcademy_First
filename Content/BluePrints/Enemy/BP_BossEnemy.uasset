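; Boss enemy Blueprint with a two-fist rocket punch attack aimed at the player.
; DoRocketAiming marks two staggered, side-offset target points near the player with circle indicators.
; DoRocketPunchL/R events lerp hidden fist components by timeline from BeginPlay-cached transforms to those targets, then spawn explosions, sphere-trace to damage TPSPlayer and hide the fists.
; Left/right naming is crossed: DoRocketPunchR moves LeftPunch, and its reset uses RightTarget rather than a hand origin.
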(event Custom|RAiming
  (bind _returnvalue (Game|Player|GetPlayerPawn 0))
  (bind _returnvalue_2 (Transformation|GetActorTransform _returnvalue))
  (bind _output_get (Variables|Default|SetRightTarget (Math|Transform|MakeTransform (+ (+ (.location _returnvalue_2) (Variables|Default|GetPlayerLen)) (* (Variables|Default|GetpunchGap) (Transformation|GetActorRightVector))) (.rotation _returnvalue_2) (.scale _returnvalue_2))))
  (bind _returnvalue_3 (Game|SpawnActorfromClass "/Game/BluePrints/Enemy/Indicator/BP_CircleIndicator.BP_CircleIndicator_C" _output_get "Undefined" "MultiplyWithRoot" 0 0))
  (Variables|/Script/Gunfire.SkillIndicator|SetCastingTime _returnvalue_3 1.3)
  (Variables|/Script/Gunfire.SkillIndicator|SetDestroyTime _returnvalue_3 1.3)
  (Transformation|SetActorScale3D _returnvalue_3 (Math|Conversions|ToVector(Float) 12.0)))

(event EventBeginPlay
  ;[1 1 1] 왼팔 오른팔 본의 위치를 기록한다.
  (Transformation|SetRelativeTransform (Variables|Default|GetLeftPunch) (Variables|Default|GetRightHandOrigin) false false)
  (Transformation|SetRelativeTransform (Variables|Default|GetRightPunch) (Variables|Default|GetLeftHandOrigin) false false)
  (Variables|Default|SetbFire false)
  (Variables|Default|SetWorldTransformL (Transformation|GetWorldTransform (Variables|Default|GetRightPunch)))
  (Variables|Default|SetWorldTransformR (Transformation|GetWorldTransform (Variables|Default|GetLeftPunch)))
  (Rendering|SetVisibility (Variables|Default|GetLeftPunch) false false))

(event EventDoRocketAiming
  (bind _returnvalue (Game|Player|GetPlayerPawn 0))
  (bind _returnvalue_2 (Transformation|GetActorTransform _returnvalue))
  (bind _output_get (Variables|Default|SetLeftTarget (Math|Transform|MakeTransform (- (+ (.location _returnvalue_2) (Variables|Default|GetPlayerLen)) (* (Variables|Default|GetpunchGap) (Transformation|GetActorRightVector))) (.rotation _returnvalue_2) (.scale _returnvalue_2))))
  (bind _returnvalue_3 (Game|SpawnActorfromClass "/Game/BluePrints/Enemy/Indicator/BP_CircleIndicator.BP_CircleIndicator_C" _output_get "Undefined" "MultiplyWithRoot" 0 0))
  (Variables|/Script/Gunfire.SkillIndicator|SetCastingTime _returnvalue_3 1.3)
  (Variables|/Script/Gunfire.SkillIndicator|SetDestroyTime _returnvalue_3 1.3)
  (Transformation|SetActorScale3D _returnvalue_3 (Math|Conversions|ToVector(Float) 12.0))
  (Utilities|Time|SetTimerbyEvent (delegate Custom|RAiming) 0.5))

(event EventDoRocketPunchL
  (bind _rightpunch (Variables|Default|GetRightPunch))
  (bind _lefttarget (Variables|Default|GetLeftTarget))
  (bind _rightpunch_2 (Variables|Default|GetRightPunch))
  (Rendering|SetVisibility _rightpunch_2 true false)
  (Variables|Default|SetbFireLeft true)
  (Audio|PlaySoundatLocation "/Game/BluePrints/EnemySFX/Lizard_Wield.Lizard_Wield" (Transformation|GetWorldLocation _rightpunch_2) "0, 0, 0" 1.0 1.0 0.0 0 0 0 0)
  (bind _newtrack_0 (Timeline|Timeline Play)
    (:Update
      (Transformation|SetWorldLocation (Variables|Default|GetRightPunch) (.location (Math|Transform|Lerp(Transform) (Variables|Default|GetWorldTransformL) (Variables|Default|GetLeftTarget) _newtrack_0)) false false))
    (:Finished
      (Game|SpawnActorfromClass "/Game/BluePrints/Enemy/Pattern/BP_PunchExplosion.BP_PunchExplosion_C" (Variables|Default|GetLeftTarget) "Undefined" "MultiplyWithRoot" 0 0)
      (bind _outhits (Collision|MultiSphereTraceByChannel (.location _lefttarget) (.location _lefttarget) 6e+02 "TraceTypeQuery1" false 0 "None"))
      (bind _array_element (Utilities|Array|ForEachLoopwithBreak _outhits :!label _label)
        (:LoopBody
          (if (.bBlockingHit (Collision|BreakHitResult _array_element))
            (bind _astpsplayer (Utilities|Casting|CastToTPSPlayer (.HitActor (Collision|BreakHitResult _array_element))))
            (Game|Damage|ApplyDamage _astpsplayer 5e+01 0 0)
            (goto _label Break)))
        (:Completed
          (Variables|Default|SetbFireLeft false)
          (Transformation|SetRelativeTransform _rightpunch (Variables|Default|GetLeftHandOrigin) false false)
          (Rendering|SetVisibility _rightpunch false false)
          (Audio|PlaySoundatLocation "/Game/BluePrints/EnemySFX/BrokenRock.BrokenRock" (Transformation|GetWorldLocation _rightpunch) "0, 0, 0" 1.0 1.0 0.0 0 0 0 0))))))

(event EventDoRocketPunchR
  (bind _leftpunch (Variables|Default|GetLeftPunch))
  (bind _leftpunch_2 (Variables|Default|GetLeftPunch))
  (bind _righttarget (Variables|Default|GetRightTarget))
  (Rendering|SetVisibility _leftpunch_2 true false)
  (Variables|Default|SetbFireRight true)
  (Audio|PlaySoundatLocation "/Game/BluePrints/EnemySFX/Lizard_Wield.Lizard_Wield" (Transformation|GetWorldLocation _leftpunch_2) "0, 0, 0" 1.0 1.0 0.0 0 0 0 0)
  (bind _newtrack_0 (Timeline|Fire PlayFromStart)
    (:Update
      (Transformation|SetWorldTransform (Variables|Default|GetLeftPunch) (Math|Transform|MakeTransform (.location (Math|Transform|Lerp(Transform) (Variables|Default|GetWorldTransformR) (Variables|Default|GetRightTarget) _newtrack_0)) (.rotation (Variables|Default|GetWorldTransformR)) "1.000000,1.000000,1.000000") false false))
    (:Finished
      (Game|SpawnActorfromClass "/Game/BluePrints/Enemy/Pattern/BP_PunchExplosion.BP_PunchExplosion_C" (Variables|Default|GetRightTarget) "Undefined" "MultiplyWithRoot" 0 0)
      (bind _outhits (Collision|MultiSphereTraceByChannel (.location _righttarget) (.location _righttarget) 6e+02 "TraceTypeQuery1" false 0 "None"))
      (bind _array_element (Utilities|Array|ForEachLoopwithBreak _outhits :!label _label)
        (:LoopBody
          (if (.bBlockingHit (Collision|BreakHitResult _array_element))
            (bind _astpsplayer (Utilities|Casting|CastToTPSPlayer (.HitActor (Collision|BreakHitResult _array_element))))
            (Game|Damage|ApplyDamage _astpsplayer 5e+01 0 0)
            (goto _label Break)))
        (:Completed
          (Variables|Default|SetbFireRight false)
          (Transformation|SetRelativeTransform _leftpunch (Variables|Default|GetRightTarget) false false)
          (Rendering|SetVisibility _leftpunch false false)
          (Audio|PlaySoundatLocation "/Game/BluePrints/EnemySFX/BrokenRock.BrokenRock" (Transformation|GetWorldLocation _leftpunch) "0, 0, 0" 1.0 1.0 0.0 0 0 0 0))))))

(fn ConstructionScript)