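; BP_DamageAmt is a floating damage number actor that shows a hit amount as a world-space widget.
; On BeginPlay it enables custom depth stencil on the widget, passes DmgAmt to WBP_DamageText, and picks a random nearby end point.
; The MoveText timeline lerps the actor to that point, then destroys it.
; Tick billboards the widget toward the player camera.
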(event EventBeginPlay
  (Utilities|FlowControl|Sequence
    (:then_0
      (Rendering|SetRenderCustomDepth (Variables|Default|GetWidget) true)
      (Rendering|SetCustomDepthStencilValue (Variables|Default|GetWidget) 255))
    (:then_1
      (bind _aswbp_damage_text (Utilities|Casting|CastToWBP_DamageText (UserInterface|GetWidget (Variables|Default|GetWidget))))
      (Variables|/Game/BluePrints/Enemy/WBP_DamageText.WBP_DamageText_C|SetDmgAmt _aswbp_damage_text (Variables|Default|GetDmgAmt))
      (bind _output_get (Variables|Default|SetStartLoc (Transformation|GetActorLocation)))
      (Variables|Default|SetEndLoc (+ _output_get (Math|Vector|MakeVector (Math|Random|RandomFloatinRange -2.5e+02 2.5e+02) (Math|Random|RandomFloatinRange -2.5e+02 2.5e+02) (Math|Random|RandomFloatinRange -2.5e+02 2.5e+02))))
      (bind _move_track (Timeline|MoveText Play)
        (:Update
          (Transformation|SetActorLocation (Math|Vector|Lerp(Vector) (Variables|Default|GetStartLoc) (Variables|Default|GetEndLoc) _move_track) false false))
        (:Finished
          (Actor|DestroyActor))))))

(event EventTick
  (params (DeltaSeconds :type Float%20%28single-precision%29))
  ;[1 1 1] Target-me로 HP Widget가 돌아가도록 빌보드 처리
  (Transformation|SetWorldRotation (Variables|Default|GetWidget) (Class|KismetMathLibrary|QuatRotator (Math|Conversions|ToQuaternion(Rotator) (- (Transformation|GetActorLocation (Game|GetPlayerCameraManager 0)) (Transformation|GetWorldLocation (Variables|Default|GetWidget))))) false false))

(fn ConstructionScript)