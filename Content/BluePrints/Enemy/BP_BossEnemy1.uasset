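; Boss enemy actor with a two-fisted rocket punch attack aimed at the player.
; DoRocketPunch poses the hands, marks two spots either side of an offset from the player with circle indicators, then launches after a delay.
; Tick flies both hands to their targets; when the left arrives, both explode, hide and damage TPSPlayer through sphere traces.
; A timer set at launch restores and reveals the hands.
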(event Custom|FirePunch
  (Variables|Default|SetbFire true)
  (Utilities|Time|SetTimerbyEvent (delegate Custom|FireEnd) 2.0))

(event Custom|FireEnd
  (Variables|Default|SetbFire false)
  (Transformation|SetRelativeTransform (Variables|Default|GetRightHand) (Variables|Default|GetRightHandOrigin) false false)
  (Transformation|SetRelativeTransform (Variables|Default|GetLeftHand) (Variables|Default|GetLeftHandOrigin) false false)
  (Variables|Default|SetbFire false)
  (Rendering|SetVisibility (Variables|Default|GetLeftHand) true false))

(event EventBeginPlay
  (Transformation|SetRelativeTransform (Variables|Default|GetRightHand) (Variables|Default|GetRightHandOrigin) false false)
  (Transformation|SetRelativeTransform (Variables|Default|GetLeftHand) (Variables|Default|GetLeftHandOrigin) false false)
  (Variables|Default|SetbFire false))

(event Collision|EventActorBeginOverlap
  (params (OtherActor :type Actor%20Object%20Reference)))

(event EventTick
  (params (DeltaSeconds :type Float%20%28single-precision%29))
  (bind _returnvalue (Utilities|Time|GetWorldDeltaSeconds))
  (bind _returnvalue_2 (Utilities|Time|GetWorldDeltaSeconds))
  (bind _punchspeed (Variables|Default|GetPunchSpeed))
  (bind _lefthand (Variables|Default|GetLeftHand))
  (bind _righthand (Variables|Default|GetRightHand))
  (bind _lefttarget (Variables|Default|GetLeftTarget))
  (bind _righttarget (Variables|Default|GetRightTarget))
  (bind _punchspeed_2 (Variables|Default|GetPunchSpeed))
  (bind _returnvalue_3 (Transformation|GetWorldLocation _righthand))
  (bind _returnvalue_4 (Transformation|GetWorldLocation _lefthand))
  (bind _returnvalue_5 (- (.location _lefttarget) _returnvalue_4))
  (bind _returnvalue_6 (- (.location _righttarget) _returnvalue_3))
  (bind _returnvalue_7 (Math|Vector|Normalize _returnvalue_5))
  (bind _returnvalue_8 (Math|Vector|Normalize _returnvalue_6))
  (bind _returnvalue_9 (* _returnvalue_8 _punchspeed_2 _returnvalue))
  (bind _returnvalue_10 (* _returnvalue_7 _punchspeed _returnvalue_2))
  (bind _returnvalue_11 (+ _returnvalue_4 _returnvalue_10))
  (bind _returnvalue_12 (+ _returnvalue_3 _returnvalue_9))
  (if (Variables|Default|GetbFire)
    (Transformation|SetWorldLocation _righthand _returnvalue_12 false false)
    (Transformation|SetWorldLocation _lefthand _returnvalue_11 false false)
    (if (< (Math|Vector|VectorLength (- _returnvalue_11 (.location _lefttarget))) 1e+02)
      (Variables|Default|SetbFire false)
      (Utilities|FlowControl|Sequence
        (:then_0
          (Game|SpawnActorfromClass "/Game/BluePrints/Enemy/Pattern/BP_PunchExplosion.BP_PunchExplosion_C" (Variables|Default|GetRightTarget) "Undefined" "MultiplyWithRoot" 0 0)
          (Game|SpawnActorfromClass "/Game/BluePrints/Enemy/Pattern/BP_PunchExplosion.BP_PunchExplosion_C" (Variables|Default|GetLeftTarget) "Undefined" "MultiplyWithRoot" 0 0)
          (Rendering|SetVisibility (Variables|Default|GetRightHand) false false)
          (bind _outhits (Collision|MultiSphereTraceByChannel _returnvalue_12 _returnvalue_12 7e+02 "TraceTypeQuery1" false 0 "None"))
          (bind _array_element (Utilities|Array|ForEachLoopwithBreak _outhits :!label _label)
            (:LoopBody
              (if (.bBlockingHit (Collision|BreakHitResult _array_element))
                (bind _astpsplayer (Utilities|Casting|CastToTPSPlayer (.HitActor (Collision|BreakHitResult _array_element))))
                (Game|Damage|ApplyDamage _astpsplayer 5e+01 0 0)
                (goto _label Break)))))
        (:then_1
          (bind _outhits_2 (Collision|MultiSphereTraceByChannel _returnvalue_11 _returnvalue_11 6e+02 "TraceTypeQuery1" false 0 "None"))
          (bind _array_element_2 (Utilities|Array|ForEachLoopwithBreak _outhits_2 :!label _label_2)
            (:LoopBody
              (if (.bBlockingHit (Collision|BreakHitResult _array_element_2))
                (bind _astpsplayer_2 (Utilities|Casting|CastToTPSPlayer (.HitActor (Collision|BreakHitResult _array_element_2))))
                (Game|Damage|ApplyDamage _astpsplayer_2 5e+01 0 0)
                (goto _label_2 Break)))))))))

(event EventDoRocketPunch
  (bind _returnvalue (Transformation|GetActorRightVector))
  (bind _returnvalue_2 (Game|Player|GetPlayerPawn 0))
  (bind _playerlen (Variables|Default|GetPlayerLen))
  (bind _punchgap (Variables|Default|GetpunchGap))
  (bind _returnvalue_3 (Transformation|GetActorTransform _returnvalue_2))
  (bind _returnvalue_4 (* _punchgap _returnvalue))
  (bind _returnvalue_5 (+ (.location _returnvalue_3) _playerlen))
  (Transformation|SetRelativeTransform (Variables|Default|GetRightHand) (Variables|Default|GetRightPuchReady) false false)
  (Transformation|SetRelativeTransform (Variables|Default|GetLeftHand) (Variables|Default|GetLeftPunchReady) false false)
  (bind _output_get (Variables|Default|SetRightTarget (Math|Transform|MakeTransform (+ _returnvalue_5 _returnvalue_4) (.rotation _returnvalue_3) (.scale _returnvalue_3))))
  (bind _output_get_2 (Variables|Default|SetLeftTarget (Math|Transform|MakeTransform (- _returnvalue_5 _returnvalue_4) (.rotation _returnvalue_3) (.scale _returnvalue_3))))
  (bind _returnvalue_6 (Game|SpawnActorfromClass "/Game/BluePrints/Enemy/Indicator/BP_CircleIndicator.BP_CircleIndicator_C" _output_get "Undefined" "MultiplyWithRoot" 0 0))
  (Transformation|SetActorScale3D _returnvalue_6 (Math|Conversions|ToVector(Float) 12.0))
  (bind _returnvalue_7 (Game|SpawnActorfromClass "/Game/BluePrints/Enemy/Indicator/BP_CircleIndicator.BP_CircleIndicator_C" _output_get_2 "Undefined" "MultiplyWithRoot" 0 0))
  (Transformation|SetActorScale3D _returnvalue_7 (Math|Conversions|ToVector(Float) 12.0))
  (Utilities|Time|SetTimerbyEvent (delegate Custom|FirePunch) 2.0))

(fn ConstructionScript)