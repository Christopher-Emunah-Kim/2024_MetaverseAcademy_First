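; BP_Door is a double door that slides open when the TPSPlayer enters its trigger box.
; The overlap stores both door actors' positions, starts a camera shake on that player's controller and plays two sounds at the door.
; A timeline then lerps each door by its open offset from the stored position and sets Open when finished, blocking later triggers; no closing logic exists.
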(event OnActorBeginOverlap(TriggerBox)
  (params (OverlappedActor :type Actor%20Object%20Reference) (OtherActor :type Actor%20Object%20Reference))
  (bind _returnvalue (Math|Vector|MakeVector 0.0 0.0 0.0))
  (bind _returnvalue_2 (Transformation|GetActorLocation))
  (bind _leftdoor (Variables|Default|GetLeftDoor))
  (bind _rightdoor (Variables|Default|GetRightDoor))
  (if (not (Variables|Default|GetbOpen))
    (bind _astpsplayer (Utilities|Casting|CastToTPSPlayer OtherActor))
    (Utilities|IsValid _leftdoor
      (:Is%20Valid
        (Utilities|IsValid _rightdoor
          (:Is%20Valid
            (Variables|Default|SetOrigLeft (Transformation|GetActorLocation _leftdoor))
            (Variables|Default|SetOrigRight (Transformation|GetActorLocation _rightdoor))
            (bind _asplayer_controller (Utilities|Casting|CastToPlayerController (Pawn|GetController _astpsplayer)))
            (Game|Feedback|ClientStartCameraShake _asplayer_controller "/Game/BluePrints/Door/BP_MyCameraShake.BP_MyCameraShake_C" 1.0 "CameraLocal" "0, 0, 0")
            (Audio|PlaySoundatLocation "/Game/BluePrints/EnemySFX/DoorEffect.DoorEffect" _returnvalue_2 "0, 0, 0" 1.0 1.0 0.0 0 0 0 0)
            (Audio|PlaySoundatLocation "/Game/BluePrints/EnemySFX/GATE_Metal_Open_02_Dark_stereo.GATE_Metal_Open_02_Dark_stereo" _returnvalue_2 "0, 0, 0" 1.0 1.0 0.0 0 0 0 0)
            (bind _newtrack_0 (Timeline|Timeline Play)
              (:Update
                (Transformation|SetActorLocation (Variables|Default|GetLeftDoor) (+ (Math|Vector|Lerp(Vector) _returnvalue (Variables|Default|GetLeftOpenPos) _newtrack_0) (Variables|Default|GetOrigLeft)) false false)
                (Transformation|SetActorLocation (Variables|Default|GetRightDoor) (+ (Math|Vector|Lerp(Vector) _returnvalue (Variables|Default|GetRightOpenPos) _newtrack_0) (Variables|Default|GetOrigRight)) false false))
              (:Finished
                (Variables|Default|SetbOpen true)))))))))

(event EventBeginPlay)

(event Collision|EventActorBeginOverlap
  (params (OtherActor :type Actor%20Object%20Reference)))

(fn ConstructionScript)