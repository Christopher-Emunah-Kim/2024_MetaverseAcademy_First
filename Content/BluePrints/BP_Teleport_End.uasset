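; BP_Teleport_End is a level-end trigger that shows the victory screen when the player enters its box.
; On overlap with a TPSPlayer, it pauses the game and removes all top-level widgets from their parent.
; It then creates WBP_VictoryUI, adds it to the viewport, switches to UI-only input focused on it, and shows the mouse cursor.
; Despite the name, no teleport logic is present.
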(event OnComponentBeginOverlap(Box)
  (params (OverlappedComponent :type Primitive%20Component%20Object%20Reference) (OtherActor :type Actor%20Object%20Reference) (OtherComp :type Primitive%20Component%20Object%20Reference) (OtherBodyIndex :type Integer) (bFromSweep :type Boolean) (SweepResult :type Hit%20Result%20Structure%20%28by%20ref%29))
  (bind _returnvalue (Game|Player|GetPlayerPawn 0))
  (bind _playerstate (Variables|/Script/Engine.Pawn|GetPlayerState _returnvalue))
  (bind _returnvalue_2 (Game|GetPlayerController _playerstate))
  (Utilities|Casting|CastToTPSPlayer OtherActor)
  ;[1 1 1] 기존 UI들의 가시성을 해제하고 승리 UI를 출력한다(마우스커서ON)
  (Game|SetGamePaused true)
  (bind _foundwidgets (Widget|GetAllWidgetsOfClass "/Script/UMG.UserWidget" true))
  (Widget|RemovefromParent _foundwidgets)
  (bind _returnvalue_3 (UserInterface|CreateWidget "/Game/BluePrints/WBP_VictoryUI.WBP_VictoryUI_C"))
  (UserInterface|Viewport|AddtoViewport _returnvalue_3 0)
  (Input|SetInputModeUIOnly _returnvalue_2 _returnvalue_3 "DoNotLock" false)
  (Variables|/Script/Engine.PlayerController|SetbShowMouseCursor _returnvalue_2 true)
  (Development|PrintString "clear"))

(event EventBeginPlay)

(event Collision|EventActorBeginOverlap
  (params (OtherActor :type Actor%20Object%20Reference)))

(event EventTick
  (params (DeltaSeconds :type Float%20%28single-precision%29)))

(fn ConstructionScript)