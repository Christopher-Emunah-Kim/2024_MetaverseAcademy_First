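; BP_TPSPlayer is the third-person shooter player Blueprint, with a small event graph for hit feedback and level restart.
; DamageIndicator creates a WBP_HitCircle widget from the player and enemy location and adds it to the viewport.
; The 0 key reloads the current level by name.
; Unconnected leftover nodes cover sniper zoom via camera FOV, HUD, restart and damage widget creation, and a debug hit sphere, none of which run.
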(event EventBeginPlay)

(event Collision|EventActorBeginOverlap
  (params (OtherActor :type Actor%20Object%20Reference)))

(event EventTick
  (params (DeltaSeconds :type Float%20%28single-precision%29)))

(event EventDamageIndicator
  (params (enemyLocation :type Vector :default "0, 0, 0"))
  (bind _returnvalue (UserInterface|CreateWidget "/Game/BluePrints/WBP_HitCircle.WBP_HitCircle_C" (Game|GetPlayerController 0) self enemyLocation))
  (UserInterface|Viewport|AddtoViewport _returnvalue 0))

(event Input|KeyboardEvents|0
  (params (Key :type Key%20Structure :default "None"))
  (:Pressed
    (bind _returnvalue (Game|GetCurrentLevelName true))
    (Game|OpenLevel(byName) (Utilities|String|StringToName _returnvalue))))

(fn ConstructionScript)